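; Hospital double door Blueprint that swings both doors open on overlap and closes them when the overlap ends.
; Two collision boxes each drive their own timeline, DoorsOpening or Timeline, which sets the yaw of DoorA and DoorB from separate tracks.
; A shared Open flag blocks a second opening, while leaving either box clears it and reverses that box's timeline without any check.
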(event `self.CollisionBox1.OnComponentBeginOverlap`
  (params (OverlappedComponent :type "PrimitiveComponent Object Reference") (OtherActor :type "Actor Object Reference") (OtherComp :type "PrimitiveComponent Object Reference") (OtherBodyIndex :type Integer) (bFromSweep :type Boolean) (SweepResult :type "HitResult Structure (by ref)"))
  (if (not (`self.Open`))
    (set `self.Open` true)
    (bind (_direction _door_a_opening _door_b_opening) (`Timeline|Doors Opening` :!via `PlayFromStart` :!label _label)
      (:`Update`
        (`SceneComponent.K2_SetRelativeRotation` (`self.DoorA`) (`KismetMathLibrary.MakeRotator` 0.0 0.0 _door_a_opening) false false)
        (`SceneComponent.K2_SetRelativeRotation` (`self.DoorB`) (`KismetMathLibrary.MakeRotator` 0.0 0.0 _door_b_opening) false false)))))

(event `self.CollisionBox1.OnComponentEndOverlap`
  (params (OverlappedComponent :type "PrimitiveComponent Object Reference") (OtherActor :type "Actor Object Reference") (OtherComp :type "PrimitiveComponent Object Reference") (OtherBodyIndex :type Integer))
  (set `self.Open` false)
  (goto _label :!via `Reverse`))

(event `self.CollisionBox2.OnComponentBeginOverlap`
  (params (OverlappedComponent :type "PrimitiveComponent Object Reference") (OtherActor :type "Actor Object Reference") (OtherComp :type "PrimitiveComponent Object Reference") (OtherBodyIndex :type Integer) (bFromSweep :type Boolean) (SweepResult :type "HitResult Structure (by ref)"))
  (if (not (`self.Open`))
    (set `self.Open` true)
    (bind (_direction _door_a_opening _door_b_opening) (`Timeline|Timeline` :!via `PlayFromStart` :!label _label_2)
      (:`Update`
        (`SceneComponent.K2_SetRelativeRotation` (`self.DoorA`) (`KismetMathLibrary.MakeRotator` 0.0 0.0 _door_a_opening) false false)
        (`SceneComponent.K2_SetRelativeRotation` (`self.DoorB`) (`KismetMathLibrary.MakeRotator` 0.0 0.0 _door_b_opening) false false)))))

(event `self.CollisionBox2.OnComponentEndOverlap`
  (params (OverlappedComponent :type "PrimitiveComponent Object Reference") (OtherActor :type "Actor Object Reference") (OtherComp :type "PrimitiveComponent Object Reference") (OtherBodyIndex :type Integer))
  (set `self.Open` false)
  (goto _label_2 :!via `Reverse`))

(fn `UserConstructionScript`)